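; Plinko multiplier slot actor that pays out money when a ball enters its box.
; On overlap, it adds the ball's value times Multiplier and the GameMode's MultiplayerUpgrade to GM_Plinko's Money, found through GetActorOfClass.
; Tick rewrites the text label with the upgraded multiplier.
; Hits on either yellow gem pillar sprite play a sound when the HUD's SoundsOnOff flag is false.
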(event OnComponentBeginOverlap(Box)
  (params (OverlappedComponent :type Primitive%20Component%20Object%20Reference) (OtherActor :type Actor%20Object%20Reference) (OtherComp :type Primitive%20Component%20Object%20Reference) (OtherBodyIndex :type Integer) (bFromSweep :type Boolean) (SweepResult :type Hit%20Result%20Structure%20%28by%20ref%29))
  ;[0 0.8802 0.131 0.5] Add Money to the GameMode
  (bind _aspsa_ball (Utilities|Casting|CastToPSA_Ball OtherActor)
    (:then
      (Development|PrintString (Utilities|String|ToString(Float) (* (Variables|/Game/Plinko/Sprits/PSA_Ball.PSA_Ball_C|GetMoneyBall _aspsa_ball) (* (Variables|Value|GetMultiplier) (Variables|/Game/Plinko/Blueprints/GM_Plinko.GM_Plinko_C|GetMultiplayerUpgrade (stale EventBeginPlay _asgm_plinko))))))
      (bind _asgm_plinko (Utilities|Casting|CastToGM_PlinkoClass "/Game/Plinko/Blueprints/GM_Plinko.GM_Plinko_C"))
      (bind _returnvalue (Actor|GetActorOfClass _asgm_plinko))
      (Variables|/Game/Plinko/Blueprints/GM_Plinko.GM_Plinko_C|SetMoney _returnvalue (+ (Variables|/Game/Plinko/Blueprints/GM_Plinko.GM_Plinko_C|GetMoney _returnvalue) (* (Variables|/Game/Plinko/Sprits/PSA_Ball.PSA_Ball_C|GetMoneyBall _aspsa_ball) (* (Variables|Value|GetMultiplier) (Variables|/Game/Plinko/Blueprints/GM_Plinko.GM_Plinko_C|GetMultiplayerUpgrade (stale EventBeginPlay _asgm_plinko)))))))
    (:CastFailed
      (Development|PrintString "CastFaield" true true "(R=1.000000,G=0.012455,B=0.000000,A=1.000000)"))))

(event OnComponentHit(PillerGemYellow_Sprite2)
  (params (HitComponent :type Primitive%20Component%20Object%20Reference) (OtherActor :type Actor%20Object%20Reference) (OtherComp :type Primitive%20Component%20Object%20Reference) (NormalImpulse :type Vector :default "0, 0, 0") (Hit :type Hit%20Result%20Structure%20%28by%20ref%29))
  (if (not (Variables|/Game/Plinko/UserInterface/HUD_Plinko.HUD_Plinko_C|GetSoundsOn/Off (stale EventBeginPlay _ashud_plinko)))
    (Audio|PlaySound2D "/Game/Plinko/Audio/HitSoundEffect.HitSoundEffect" 1.0 1.0 0.0 0 0)))

(event OnComponentHit(PillerGemYellow_Sprite)
  (params (HitComponent :type Primitive%20Component%20Object%20Reference) (OtherActor :type Actor%20Object%20Reference) (OtherComp :type Primitive%20Component%20Object%20Reference) (NormalImpulse :type Vector :default "0, 0, 0") (Hit :type Hit%20Result%20Structure%20%28by%20ref%29))
  (if (not (Variables|/Game/Plinko/UserInterface/HUD_Plinko.HUD_Plinko_C|GetSoundsOn/Off (stale EventBeginPlay _ashud_plinko)))
    (Audio|PlaySound2D "/Game/Plinko/Audio/HitSoundEffect.HitSoundEffect" 1.0 1.0 0.0 0 0)))

(event EventBeginPlay
  (bind _asgm_plinko (Utilities|Casting|CastToGM_Plinko (Game|GetGameMode)))
  (bind _ashud_plinko (Utilities|Casting|CastToHUD_Plinko (HUD|GetHUD (Game|GetPlayerController 0)))))

(event EventTick
  (params (DeltaSeconds :type Float%20%28single-precision%29))
  (Rendering|Components|TextRender|SetText (Variables|Default|GetTextRender) (Utilities|Text|ToText(String) (Utilities|String|Append (Utilities|String|ToString(Text) (Utilities|Text|ToText(Float) (* (Variables|Value|GetMultiplier) (Variables|/Game/Plinko/Blueprints/GM_Plinko.GM_Plinko_C|GetMultiplayerUpgrade (stale EventBeginPlay _asgm_plinko))) "HalfToEven")) "x"))))

(fn ConstructionScript)